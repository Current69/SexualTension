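; Melee hammer pickup that spins and bobs until it is equipped.
; Tick rotates the skeletal mesh and flips its hover direction at upper and lower height limits, with movement applied per frame without delta-time scaling.
; EquipSphere overlaps with BP_Character toggle that character's equip HUD and the CanEquip flag.
; The sphere destroys itself on end overlap once Equipped, which is set outside these graphs.
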(event OnComponentBeginOverlap(equipSphere)
  (params (OverlappedComponent :type Primitive%20Component%20Object%20Reference) (OtherActor :type Actor%20Object%20Reference) (OtherComp :type Primitive%20Component%20Object%20Reference) (OtherBodyIndex :type Integer) (bFromSweep :type Boolean) (SweepResult :type Hit%20Result%20Structure%20%28by%20ref%29))
  ;[1 1 1] Picking up the hammer
  (bind _asbp_character (Utilities|Casting|CastToBP_Character OtherActor))
  (Development|PrintString "OVERLAPPED!")
  (Utilities|FlowControl|Sequence
    (:then_0
      (Utilities|FlowControl|DoOnce false
        (:Completed
          (UserInterface|Viewport|AddtoViewport (Variables|/Game/Blueprint/BP_Character.BP_Character_C|GetequipHud _asbp_character) 0))))
    (:then_1
      (Widget|SetVisibility (Variables|/Game/Blueprint/BP_Character.BP_Character_C|GetequipHud _asbp_character) "Visible")
      (Variables|Default|SetcanEquip true))))

(event OnComponentEndOverlap(equipSphere)
  (params (OverlappedComponent :type Primitive%20Component%20Object%20Reference) (OtherActor :type Actor%20Object%20Reference) (OtherComp :type Primitive%20Component%20Object%20Reference) (OtherBodyIndex :type Integer))
  ;[1 1 1] Destroy the pickup collision
  (bind _asbp_character (Utilities|Casting|CastToBP_Character OtherActor))
  (Development|PrintString "End overlap")
  (Widget|SetVisibility (Variables|/Game/Blueprint/BP_Character.BP_Character_C|GetequipHud _asbp_character) "Hidden")
  (Variables|Default|SetcanEquip false)
  (if (Variables|Default|Getequipped)
    (Components|DestroyComponent (Variables|Default|GetequipSphere))))

(event EventTick
  (params (DeltaSeconds :type Float%20%28single-precision%29))
  (bind _skeletalmesh (Variables|Default|GetSkeletalMesh))
  (bind _relativelocation (Variables|/Script/Engine.SceneComponent|GetRelativeLocation _skeletalmesh))
  ;[1 1 1] Spinny hammer pickup
  (if (not (Variables|Default|Getequipped))
    (Transformation|AddLocalRotation (Variables|Default|GetSkeletalMesh) "0,3.000000, 0" false false)
    (if (>= (.z _relativelocation) 1e+01)
      (Variables|Default|Sethover%20Direction (* -1 (Variables|Default|Gethover%20Direction)) :!label _label)
      (elif (<= (.z _relativelocation) -1.0)
        (goto _label)
        (else
          _)))
    (Transformation|AddRelativeLocation (Variables|Default|GetSkeletalMesh) (Math|Vector|MakeVector 0.0 0.0 (Variables|Default|Gethover%20Direction)) false true)))

(fn ConstructionScript)