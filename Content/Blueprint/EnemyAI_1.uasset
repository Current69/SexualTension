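; Enemy Blueprint that chases the player character and can be killed with a melee hammer.
; A PawnSensing sighting of BP_Character starts an AI MoveTo toward that character.
; Each begin overlap with a BP_Melee_Hammer1 subtracts fixed damage from EnemyHealth and sets EnemyDead once health runs out.
; Tick polls that flag and destroys the actor.
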(event OnSeePawn(PawnSensing)
  (params (Pawn :type Pawn%20Object%20Reference))
  (bind _asbp_character (Utilities|Casting|CastToBP_Character Pawn))
  (AI|AIMoveTo self "0, 0, 0" _asbp_character 5.0 false))

(event EventTick
  (params (DeltaSeconds :type Float%20%28single-precision%29))
  (if (Variables|Default|GetEnemyDead)
    (Actor|DestroyActor)))

(event Collision|EventActorBeginOverlap
  (params (OtherActor :type Actor%20Object%20Reference))
  (if true
    (bind _asbp_melee_hammer_1 (Utilities|Casting|CastToBP_Melee_Hammer1 OtherActor))
    (bind _output_get (Variables|Default|SetEnemyHealth (- (Variables|Default|GetEnemyHealth) 25.0)))
    (if (<= _output_get 0.0)
      (Variables|Default|SetEnemyDead true))))

(fn ConstructionScript)