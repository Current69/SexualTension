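; Game mode that starts enemy spawning and keeps the narwhal horn count.
; On BeginPlay it stores the first EnemySpawner in the level and sets a looping timer that calls its SpawnEnemy function at an interval derived from EnemiesPerSecond.
; It also adds the NarwhalPickup widget to the viewport.
; The AddNarwhalHorn event adds the passed amount to the running NarwhalHorn total.
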(event Custom|AddNarwhalHorn
  (params (Add%20Narwhal%20Horns :type Integer))
  (Variables|Default|SetNarwhalHorn (+ Add%20Narwhal%20Horns (Variables|Default|GetNarwhalHorn))))

(event EventBeginPlay
  (Utilities|FlowControl|Sequence
    (:then_0
      (bind _outactors (Actor|GetAllActorsOfClass "/Game/Blueprint/EnemySpawner.EnemySpawner_C"))
      (bind _output_get (Variables|Default|SetSpawner (Utilities|Array|Get(acopy) _outactors)))
      (Utilities|Time|SetTimerbyFunctionName _output_get "SpawnEnemy" (/ 1.0 (Variables|Default|GetEnemiesPerSecond)) true))
    (:then_1
      (bind _returnvalue (UserInterface|CreateWidget "/Game/Blueprint/Pickups/NarwhalPickup.NarwhalPickup_C"))
      (UserInterface|Viewport|AddtoViewport _returnvalue 0))))

(fn ConstructionScript)