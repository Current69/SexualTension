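; Teddy enemy AI that wanders to random nearby points, pursues the player and launches grenade projectiles.
; PawnSensing or a delayed Tick check drives the chase, moving toward the player beyond a set distance and turning to face them.
; Once shooting is enabled, delayed spawns launch grenades with an impulse along the mesh's right vector.
; Overlaps with any of four melee hammer types reduce health, and Tick destroys the enemy once dead.
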(event OnSeePawn(PawnSensing)
  (params (Pawn :type Pawn%20Object%20Reference))
  (Variables|Default|SetCanSeePlayer true)
  (bind _asbp_character (Utilities|Casting|CastToBP_Character Pawn))
  (Utilities|FlowControl|Sequence
    (:then_0
      (if (>= (Transformation|GetDistanceTo _asbp_character) (Variables|Default|GetEnemyDistance))
        (AI|AIMoveTo self "0, 0, 0" _asbp_character 1e+01 false
          (:then
            (Transformation|SetActorRotation (Math|Rotator|FindLookatRotation (Transformation|GetActorLocation) (Transformation|GetActorLocation _asbp_character)) :!label _label)
            (Variables|Default|Setspawn%20projectile true))
          (:OnSuccess
            (Variables|Default|SetCanSeePlayer false)))
        (else
          (goto _label))))
    (:then_1
      (if (Variables|Default|Getspawn%20projectile)
        (Utilities|FlowControl|Delay 3.0)
        (bind _returnvalue (Game|SpawnActorfromClass "/Game/Blueprints/grinade.grinade_C" (Transformation|GetWorldTransform (Variables|Default|GetprojectileSpawnLocation)) "Undefined" 0 0))
        (Physics|AddImpulse (Variables|/Game/Blueprints/grinade.grinade_C|GetStaticMesh _returnvalue) (* (Math|Vector|GetRightVector (Variables|Character|GetMesh)) (Variables|Default|Getshoot%20amount)) "Projectile_Spawn" true)
        (Utilities|FlowControl|Delay 1e+01)
        (Variables|Default|Setspawn%20projectile true)
        (Utilities|FlowControl|Delay 0.2)
        (Variables|Default|SetdestroyCrate true)))))

(event EventTick
  (params (DeltaSeconds :type Float%20%28single-precision%29))
  (Utilities|FlowControl|Sequence
    (:then_0
      (Utilities|FlowControl|Delay 3.0)
      (if (Variables|Default|GetCanSeePlayer)
        (Variables|Default|SetCanSeePlayer true)
        (bind _asbp_character (Utilities|Casting|CastToBP_Character (stale OnSeePawn(PawnSensing) Pawn)))
        (Utilities|FlowControl|Sequence
          (:then_0
            (if (>= (Transformation|GetDistanceTo _asbp_character) (Variables|Default|GetEnemyDistance))
              (AI|AIMoveTo self "0, 0, 0" _asbp_character 1e+01 false
                (:then
                  (Transformation|SetActorRotation (Math|Rotator|FindLookatRotation (Transformation|GetActorLocation) (Transformation|GetActorLocation _asbp_character)) :!label _label)
                  (Variables|Default|Setspawn%20projectile true))
                (:OnSuccess
                  (Variables|Default|SetCanSeePlayer false)))
              (else
                (goto _label))))
          (:then_1
            (if (Variables|Default|Getspawn%20projectile)
              (Utilities|FlowControl|Delay 3.0)
              (bind _returnvalue (Game|SpawnActorfromClass "/Game/Blueprints/grinade.grinade_C" (Transformation|GetWorldTransform (Variables|Default|GetprojectileSpawnLocation)) "Undefined" 0 0))
              (Physics|AddImpulse (Variables|/Game/Blueprints/grinade.grinade_C|GetStaticMesh _returnvalue) (* (Math|Vector|GetRightVector (Variables|Character|GetMesh)) (Variables|Default|Getshoot%20amount)) "Projectile_Spawn" true)
              (Utilities|FlowControl|Delay 1e+01)
              (Variables|Default|Setspawn%20projectile true)
              (Utilities|FlowControl|Delay 0.2)
              (Variables|Default|SetdestroyCrate true))))
        (else
          (AI|AIMoveTo self (.RandomLocation (AI|Navigation|GetRandomReachablePointinRadius (Transformation|GetActorLocation) 5e+02 0 0)) 0 5.0 false))))
    (:then_1
      (if (Variables|Default|GetEnemy%20Dead)
        (Actor|DestroyActor)))))

(event Collision|EventActorBeginOverlap
  (params (OtherActor :type Actor%20Object%20Reference))
  (if true
    (Utilities|FlowControl|Sequence
      (:then_0
        (bind _asbp_melee_hammer_1 (Utilities|Casting|CastToBP_Melee_Hammer1 OtherActor)))
      (:then_1
        (bind _asbp_melee_hammer_2 (Utilities|Casting|CastToBP_Melee_Hammer2 OtherActor)))
      (:then_2
        (bind _asbp_melee_hammer_3 (Utilities|Casting|CastToBP_Melee_Hammer3 OtherActor)))
      (:then_3
        (bind _asbp_melee_hammer_4 (Utilities|Casting|CastToBP_Melee_Hammer4 OtherActor))))
    (bind _output_get (Variables|Default|SetEnemy%20Health (- (Variables|Default|GetEnemy%20Health) 25.0)))
    (if (<= _output_get 0.0)
      (Variables|Default|SetEnemy%20Dead true))))

(fn ConstructionScript)