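; Observatory platform that freezes BP_Character on entering its trigger, then rises once while celebration effects play.
; The first overlap spawns balloon emitters and runs the RisingPlatform timeline, adding VerticalRise to the actor's current location each update.
; When the rise finishes, an endless delayed loop cycles through four fireworks stages at hardcoded world positions, randomly picking one of four particle systems per stage.
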(event OnComponentBeginOverlap(Trigger)
  (params (OverlappedComponent :type Primitive%20Component%20Object%20Reference) (OtherActor :type Actor%20Object%20Reference) (OtherComp :type Primitive%20Component%20Object%20Reference) (OtherBodyIndex :type Integer) (bFromSweep :type Boolean) (SweepResult :type Hit%20Result%20Structure%20%28by%20ref%29))
  ;[1 1 1] Set "Frozen" to True on BP_Character, "Triggered" to True on Self, to Disallow Movement
  (bind _asbp_character (Utilities|Casting|CastToBP_Character OtherActor))
  (Variables|/Game/Blueprint/BP_Character.BP_Character_C|SetFrozen _asbp_character true)
  (if (not (Variables|Default|GetTriggered))
    (Variables|Default|SetTriggered true)
    ;[1 1 1] Activate Balloon Circles
    (Effects|SpawnEmitteratLocation "/Game/Particles/Balloons/PS_Balloons.PS_Balloons" "-2474.388184,6897.040527,874.991760" "0, 0, 0" "1.000000,1.000000,1.000000" false)
    (Effects|SpawnEmitteratLocation "/Game/Particles/Balloons/PS_Balloons.PS_Balloons" "2148.082520,6764.185547,874.992737" "0, 0, 0" "1.000000,1.000000,1.000000" false)
    (Effects|SpawnEmitteratLocation "/Game/Particles/Balloons/PS_Balloons.PS_Balloons" "2148.082520,2325.114258,874.992981" "0, 0, 0" "1.000000,1.000000,1.000000" false)
    (bind _verticalrise (Timeline|RisingPlatform PlayFromStart)
      (:Update
        (Transformation|SetActorLocation (+ _verticalrise (Transformation|GetActorLocation)) false false))
      (:Finished
        (switch int (Math|Random|RandomIntegerinRange 0 3) :!label _label
          (:0
            (Effects|SpawnEmitteratLocation "/Game/Particles/Fireworks/PS_Fireworks.PS_Fireworks" "1728.377930,5202.106934,874.992981" "0.000000,-90.000000,0.000000")
            (Effects|SpawnEmitteratLocation "/Game/Particles/Fireworks/PS_Fireworks.PS_Fireworks" "-2198.548340,5156.421387,874.992920" "0.000000,90.000000,0.000000"))
          (:1
            (Effects|SpawnEmitteratLocation "/Game/Particles/Fireworks/PS_Fireworks2.PS_Fireworks2" "1728.377930,5202.106934,874.992981" "0.000000,-90.000000,0.000000")
            (Effects|SpawnEmitteratLocation "/Game/Particles/Fireworks/PS_Fireworks2.PS_Fireworks2" "-2198.548340,5156.421387,874.992920" "0.000000,90.000000,0.000000"))
          (:2
            (Effects|SpawnEmitteratLocation "/Game/Particles/Fireworks/PS_Fireworks3.PS_Fireworks3" "1728.377930,5202.106934,874.992981" "0.000000,-90.000000,0.000000")
            (Effects|SpawnEmitteratLocation "/Game/Particles/Fireworks/PS_Fireworks3.PS_Fireworks3" "-2198.548340,5156.421387,874.992920" "0.000000,90.000000,0.000000"))
          (:3
            (Effects|SpawnEmitteratLocation "/Game/Particles/Fireworks/PS_Fireworks4.PS_Fireworks4" "1728.377930,5202.106934,874.992981" "0.000000,-90.000000,0.000000")
            (Effects|SpawnEmitteratLocation "/Game/Particles/Fireworks/PS_Fireworks4.PS_Fireworks4" "-2198.548340,5156.421387,874.992920" "0.000000,90.000000,0.000000")))
        (Utilities|FlowControl|Delay 0.5)
        (switch int (Math|Random|RandomIntegerinRange 0 3)
          (:0
            (Effects|SpawnEmitteratLocation "/Game/Particles/Fireworks/PS_Fireworks.PS_Fireworks" "1147.613159,6581.855469,874.992981" "0,-45.000000, 0")
            (Effects|SpawnEmitteratLocation "/Game/Particles/Fireworks/PS_Fireworks.PS_Fireworks" "-1594.776855,3757.664551,874.992920" "0,135.000000, 0"))
          (:1
            (Effects|SpawnEmitteratLocation "/Game/Particles/Fireworks/PS_Fireworks2.PS_Fireworks2" "1147.613159,6581.855469,874.992981" "0,-45.000000, 0")
            (Effects|SpawnEmitteratLocation "/Game/Particles/Fireworks/PS_Fireworks2.PS_Fireworks2" "-1594.776855,3757.664551,874.992920" "0,135.000000, 0"))
          (:2
            (Effects|SpawnEmitteratLocation "/Game/Particles/Fireworks/PS_Fireworks3.PS_Fireworks3" "1147.613159,6581.855469,874.992981" "0,-45.000000, 0")
            (Effects|SpawnEmitteratLocation "/Game/Particles/Fireworks/PS_Fireworks3.PS_Fireworks3" "-1594.776855,3757.664551,874.992920" "0,135.000000, 0"))
          (:3
            (Effects|SpawnEmitteratLocation "/Game/Particles/Fireworks/PS_Fireworks4.PS_Fireworks4" "1147.613159,6581.855469,874.992981" "0,-45.000000, 0")
            (Effects|SpawnEmitteratLocation "/Game/Particles/Fireworks/PS_Fireworks4.PS_Fireworks4" "-1594.776855,3757.664551,874.992920" "0,135.000000, 0")))
        (Utilities|FlowControl|Delay 0.5)
        (switch int (Math|Random|RandomIntegerinRange 0 3)
          (:0
            (Effects|SpawnEmitteratLocation "/Game/Particles/Fireworks/PS_Fireworks.PS_Fireworks" "-227.910858,7162.298828,874.992981"))
          (:1
            (Effects|SpawnEmitteratLocation "/Game/Particles/Fireworks/PS_Fireworks2.PS_Fireworks2" "-227.910858,7162.298828,874.992981"))
          (:2
            (Effects|SpawnEmitteratLocation "/Game/Particles/Fireworks/PS_Fireworks3.PS_Fireworks3" "-227.910858,7162.298828,874.992981"))
          (:3
            (Effects|SpawnEmitteratLocation "/Game/Particles/Fireworks/PS_Fireworks4.PS_Fireworks4" "-227.910858,7162.298828,874.992981")))
        (Utilities|FlowControl|Delay 0.5)
        (switch int (Math|Random|RandomIntegerinRange 0 3)
          (:0
            (Effects|SpawnEmitteratLocation "/Game/Particles/Fireworks/PS_Fireworks.PS_Fireworks" "-1615.043091,6559.866699,874.992981" "0.000000,45.000000, 0")
            (Effects|SpawnEmitteratLocation "/Game/Particles/Fireworks/PS_Fireworks.PS_Fireworks" "1160.469971,3800.133301,874.992920" "0.000000,-135.000000, 0"))
          (:1
            (Effects|SpawnEmitteratLocation "/Game/Particles/Fireworks/PS_Fireworks2.PS_Fireworks2" "-1615.043091,6559.866699,874.992981" "0.000000,45.000000, 0")
            (Effects|SpawnEmitteratLocation "/Game/Particles/Fireworks/PS_Fireworks2.PS_Fireworks2" "1160.469971,3800.133301,874.992920" "0,-135.000000, 0"))
          (:2
            (Effects|SpawnEmitteratLocation "/Game/Particles/Fireworks/PS_Fireworks3.PS_Fireworks3" "-1615.043091,6559.866699,874.992981" "0.000000,45.000000, 0")
            (Effects|SpawnEmitteratLocation "/Game/Particles/Fireworks/PS_Fireworks3.PS_Fireworks3" "1160.469971,3800.133301,874.992920" "0.000000,-135.000000, 0"))
          (:3
            (Effects|SpawnEmitteratLocation "/Game/Particles/Fireworks/PS_Fireworks4.PS_Fireworks4" "-1615.043091,6559.866699,874.992981" "0.000000,45.000000, 0")
            (Effects|SpawnEmitteratLocation "/Game/Particles/Fireworks/PS_Fireworks4.PS_Fireworks4" "1160.469971,3800.133301,874.992920" "0,-135.000000, 0")))
        (Utilities|FlowControl|Delay 0.5)
        (goto _label)))))

(fn ConstructionScript)