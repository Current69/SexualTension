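; SpinTrap_Gold is a moving trap actor that damages actors overlapping it.
; On BeginPlay it stores its starting location, then a timeline drives its position as an offset from that point, without sweeping.
; An overlap passes a DoOnce gate to apply fixed damage, and a one-second delay resets the gate, giving a cooldown shared by all overlapping actors.
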(event Collision|EventActorBeginOverlap
  (params (OtherActor :type Actor%20Object%20Reference))
  (Utilities|FlowControl|DoOnce false :!label _label
    (:Completed
      (Utilities|FlowControl|Sequence
        (:then_0
          (Utilities|FlowControl|RetriggerableDelay 1.0)
          (goto _label Reset))
        (:then_1
          (Game|Damage|ApplyDamage OtherActor 25.0 0 0))))))

(event EventBeginPlay
  (Variables|Default|SetPlatformLocation (Transformation|GetActorLocation))
  (bind _movement (Timeline|Timeline_0 Play)
    (:Update
      (Transformation|SetActorLocation (+ _movement (Variables|Default|GetPlatformLocation)) false false))))

(fn ConstructionScript)