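; BP_Enemy1 is an enemy Blueprint, stored in an OLD folder, with simple health and death logic.
; While alive, each hit on DamageCollisionEnemy1 subtracts a floored constant of zero from health, so hits deal no damage as written.
; If health is at or below zero after a hit, it clears Alive and destroys only the Enemy1 component.
; A cast to BP_Melee_Hammer1 and its KillBoxHammer reference are left unconnected.
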(event OnComponentHit(damageCollisionEnemy1)
  (params (HitComponent :type Primitive%20Component%20Object%20Reference) (OtherActor :type Actor%20Object%20Reference) (OtherComp :type Primitive%20Component%20Object%20Reference) (NormalImpulse :type Vector :default "0, 0, 0") (Hit :type Hit%20Result%20Structure%20%28by%20ref%29))
  (if (Variables|Default|GetAlive)
    (Variables|Default|SetHealthEnemy1 (- (Variables|Default|GetHealthEnemy1) (Math|Float|Floor 0.0)))
    (if (<= (Variables|Default|GetHealthEnemy1) 0)
      (Variables|Default|SetAlive false)
      (Components|DestroyComponent (Variables|Default|Getenemy1)))))

(fn ConstructionScript)