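; BP_NarwhalGoldRed is a pickup that grants the player character a horn on overlap.
; From BeginPlay, a timeline offsets the actor from its starting location by a Height track.
; Overlap by a BP_Character calls AddHorn and plays a pickup sound, then after a short delay plays a second sound, spawns a sparkle burst and destroys the actor.
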(event OnComponentBeginOverlap(StaticMesh)
  (params (OverlappedComponent :type Primitive%20Component%20Object%20Reference) (OtherActor :type Actor%20Object%20Reference) (OtherComp :type Primitive%20Component%20Object%20Reference) (OtherBodyIndex :type Integer) (bFromSweep :type Boolean) (SweepResult :type Hit%20Result%20Structure%20%28by%20ref%29))
  (bind _asbp_character (Utilities|Casting|CastToBP_Character OtherActor))
  (Default|AddHorn _asbp_character)
  (Audio|PlaySoundatLocation "/Game/Sounds/PICKUP.PICKUP" (Transformation|GetActorLocation) "0, 0, 0" 0.5 1.0 0.0 0 0 0)
  (Utilities|FlowControl|Delay 0.2)
  (Audio|PlaySoundatLocation "/Game/Sounds/aaaah.aaaah" "0, 0, 0" "0, 0, 0" 3.5 1.0 0.0 0 0 0)
  (Effects|SpawnEmitteratLocation "/Game/Particles/Sparks/PS_Sparkleburst.PS_Sparkleburst" (Transformation|GetActorLocation))
  (Actor|DestroyActor))

(event EventBeginPlay
  (Variables|Default|SetLocation (Transformation|GetActorLocation))
  (bind _height (Timeline|Timeline_0 Play)
    (:Update
      (Transformation|SetActorLocation (+ (Variables|Default|GetLocation) _height) false false))))

(fn ConstructionScript)