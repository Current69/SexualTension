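; Enemy actor that turns to face a seen BP_Character and launches Grinade projectiles at it.
; Pawn sensing snaps the actor's rotation to the target and sets SpawnProjectile, which is never cleared here.
; After a delay, a Grinade spawns at ProjectileSpawnLocation and gets a velocity-change impulse along the mesh's right vector, scaled by ShootAmount.
; Further delays precede re-setting SpawnProjectile and setting DestroyCrate, which this graph never reads.
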(event OnSeePawn(PawnSensing)
  (params (Pawn :type Pawn%20Object%20Reference))
  (bind _asbp_character (Utilities|Casting|CastToBP_Character Pawn))
  (Utilities|FlowControl|Sequence
    (:then_0
      (Transformation|SetActorRotation (Math|Rotator|FindLookatRotation (Transformation|GetActorLocation) (Transformation|GetActorLocation _asbp_character)))
      (Variables|Default|Setspawn%20projectile true))
    (:then_1
      (if (Variables|Default|Getspawn%20projectile)
        (Utilities|FlowControl|Delay 3.0)
        (bind _returnvalue (Game|SpawnActorfromClass "/Game/Blueprints/grinade.grinade_C" (Transformation|GetWorldTransform (Variables|Default|GetprojectileSpawnLocation)) "Undefined" 0 0))
        (Physics|AddImpulse (Variables|/Game/Blueprints/grinade.grinade_C|GetStaticMesh _returnvalue) (* (Math|Vector|GetRightVector (Variables|Character|GetMesh)) (Variables|Default|Getshoot%20amount)) "Projectile_Spawn" true)
        (Utilities|FlowControl|Delay 1e+01)
        (Variables|Default|Setspawn%20projectile true)
        (Utilities|FlowControl|Delay 0.2)
        (Variables|Default|SetdestroyCrate true)))))

(fn ConstructionScript)