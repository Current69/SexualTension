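; Asteroid Blueprint that slowly spins its static mesh and hovers it vertically, with all motion driven per frame in Tick.
; Each tick adds a small local rotation and moves the mesh along Z by HoverDirection, negating that value at the upper height limit.
; The lower limit check has no reversal: at or below it the mesh stops moving vertically and only rotates.
; Steps are not scaled by delta time, so speed depends on frame rate.
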(event EventTick
  (params (DeltaSeconds :type Float%20%28single-precision%29))
  (bind _staticmesh (Variables|Default|GetStaticMesh))
  (bind _relativelocation (Variables|/Script/Engine.SceneComponent|GetRelativeLocation _staticmesh))
  (Transformation|AddLocalRotation (Variables|Default|GetStaticMesh) "0,0.100000, 0" false false)
  (if (>= (.z _relativelocation) 1e+01)
    (Variables|Default|SetHoverDirection (* -1.0 (Variables|Default|GetHoverDirection)))
    (Transformation|AddRelativeLocation (Variables|Default|GetStaticMesh) (Math|Vector|MakeVector 0.0 0.0 (Variables|Default|GetHoverDirection)) false false :!label _label)
    (elif (not (<= (.z _relativelocation) -1.0))
      (goto _label))))

(fn ConstructionScript)